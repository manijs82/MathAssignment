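; BP_Pawn is a pawn that sets up the HUD and watches the obstacle count to restart the level.
; On BeginPlay it creates a BP_HUD widget for the first player controller and adds it to the viewport.
; Every tick it counts all BP_Obstacle actors in the world and reopens the "Map" level when none remain or more than 30 exist.
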(event EventBeginPlay
  (bind _returnvalue (UserInterface|CreateWidget "/Game/Blueprints/BP_HUD.BP_HUD_C" (Game|GetPlayerController 0)))
  (UserInterface|Viewport|AddtoViewport _returnvalue 0))

(event EventTick
  (params (DeltaSeconds :type Float%20%28single-precision%29))
  (bind _count (CallFunction|GetObstacleCount))
  (if (or (< _count 1) (> _count 30))
    (Game|OpenLevel(byName) "Map")))

(fn ConstructionScript)

(fn GetObstacleCount
  (bind _outactors (Actor|GetAllActorsOfClass "/Game/Blueprints/BP_Obstacle.BP_Obstacle_C"))
  (return (Utilities|Array|Length _outactors)))