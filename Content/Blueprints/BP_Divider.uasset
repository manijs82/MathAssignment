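; BP_Divider is a Blueprint that moves a 2D point, Line1Start, with the WASD keys.
; BeginPlay enables player input, and key events set Up and Right.
; Tick normalizes that direction and shifts the point a fixed step each frame, independent of delta time.
; DrawSphere and DrawLine helpers render 2D debug shapes at zero height, but no graph here calls them.
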(event EventBeginPlay
  (Input|EnableInput (Game|GetPlayerController 0)))

(event EventTick
  (params (DeltaSeconds :type Float%20%28single-precision%29))
  (bind _output_get (Variables|Default|SetMoveVector (Math|Vector2D|MakeVector2D (Math|Conversions|ToFloat(Integer) (Variables|Default|GetUp)) (Math|Conversions|ToFloat(Integer) (Variables|Default|GetRight)))))
  (Variables|Default|SetLine1Start (+ (Variables|Default|GetLine1Start) (* (Class|KismetMathLibrary|NormalSafe2D _output_get 0.0) 1e+01))))

(event Input|KeyboardEvents|D
  (params (Key :type Key%20Structure :default "None"))
  (:Pressed
    (Variables|Default|SetRight 1))
  (:Released
    (Variables|Default|SetRight 0)))

(event Input|KeyboardEvents|W
  (params (Key :type Key%20Structure :default "None"))
  (:Pressed
    (Variables|Default|SetUp 1))
  (:Released
    (Variables|Default|SetUp 0)))

(event Input|KeyboardEvents|S
  (params (Key :type Key%20Structure :default "None"))
  (:Pressed
    (Variables|Default|SetUp -1))
  (:Released
    (Variables|Default|SetUp 0)))

(event Input|KeyboardEvents|A
  (params (Key :type Key%20Structure :default "None"))
  (:Pressed
    (Variables|Default|SetRight -1))
  (:Released
    (Variables|Default|SetRight 0)))

(fn ConstructionScript)

(fn DrawSphere
  (params (InVector2D :type Vector%202D%20Structure))
  (Rendering|Debug|DrawDebugSphere (Math|Conversions|ToVector(Vector2D) InVector2D) 2e+01 12 "(R=1.000000,G=1.000000,B=1.000000,A=1.000000)" 0.0))

(fn DrawLine
  (params (Start :type Vector%202D%20Structure) (End :type Vector%202D%20Structure))
  (Rendering|Debug|DrawDebugLine :LineStart (Math|Conversions|ToVector(Vector2D) Start) :LineEnd (Math|Conversions|ToVector(Vector2D) End)))